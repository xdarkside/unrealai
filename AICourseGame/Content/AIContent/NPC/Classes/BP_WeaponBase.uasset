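; BP_WeaponBase is a base NPC weapon that handles fire requests, with an empty reload event.
; Firing spawns a BP_Bullet at the Arrow component and runs a debug-drawn visibility trace along its forward vector, whose hit result is unused.
; A DoOnce gate blocks repeat shots until the cyclic-rate delay ends, when the weapon calls OnWeaponFired and resets the gate.
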(event `FireReguest`
  (bind _arrow (`self.Arrow`))
  (bind _arrow_2 (`self.Arrow`))
  (bind _returnvalue (`SceneComponent.K2_GetComponentLocation` _arrow_2))
  (`/Engine/EditorBlueprintResources/StandardMacros.DoOnce` false :!label _label
    (:`Completed`
      (`|SpawnActorFromClass` "/Game/AIContent/NPC/Classes/BP_Bullet.BP_Bullet_C" (`KismetMathLibrary.MakeTransform` (`SceneComponent.K2_GetComponentLocation` _arrow) (`SceneComponent.K2_GetComponentRotation` _arrow)) "AlwaysSpawn" "MultiplyWithRoot" null null)
      (`KismetSystemLibrary.LineTraceSingle` :`Start` _returnvalue :`End` (+ _returnvalue (* (`SceneComponent.GetForwardVector` _arrow_2) (`self.WeaponRange`))) :`TraceChannel` "TraceTypeQuery1" :`DrawDebugType` "ForDuration")
      (`KismetSystemLibrary.PrintString` "Shot")
      (`KismetSystemLibrary.Delay` (`self.CyclycRate`))
      (`self.OnWeaponFired`)
      (goto _label :!via `Reset`))))

(event `ReloadReguest`)

(fn `UserConstructionScript`)
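; BP_Guard is an AI guard NPC that spawns a weapon into its hand socket and fires it on request.
; HealthComponent events play a hit montage on damage and, on death, ragdoll the mesh and stop the AI brain logic once.
; State and aim changes are forwarded to the AnimInstance via messages, while walk speed follows AI state.
; Getters expose patrol route, team, weapon, range and death status.
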(event `self.ReceiveBeginPlay`
  (bind _returnvalue (`|SpawnActorFromClass` "/Game/AIContent/NPC/Classes/BP_WeaponBase.BP_WeaponBase_C" (`/Game/AIContent/NPC/Guard/GlobalFunctions.IdentTransform`) "AlwaysSpawn" "MultiplyWithRoot" null null))
  (set `self.Weapon` _returnvalue)
  (`self.K2_AttachToComponent` _returnvalue (`self.Mesh`) "WeaponSocket" "SnapToTarget" "SnapToTarget" "SnapToTarget" true)
  (set `self.MainMesh` (`self.Mesh`)))

(event `self.HealthComponent.TakeDamageDispatcher`
  (`KismetSystemLibrary.PrintString` (`KismetStringLibrary.Conv_DoubleToString` (`/Game/AIContent/NPC/Guard/HealthComponent.Health` (`self.HealthComponent`))))
  (`|PlayMontage` (`self.Mesh`) "/Game/AIContent/NPC/Guard/Animations/HitMontage.HitMontage"))

(event `self.HealthComponent.DeathDispetcher`
  (bind _mesh (`self.Mesh`))
  (`/Engine/EditorBlueprintResources/StandardMacros.DoOnce` false
    (:`Completed`
      (`PrimitiveComponent.SetCollisionProfileName` (`self.Mesh`) "Ragdoll" true)
      (`SkeletalMeshComponent.SetAllBodiesSimulatePhysics` _mesh true)
      (`PrimitiveComponent.WakeAllRigidBodies` _mesh)
      (`BrainComponent.StopLogic` (`AIController.BrainComponent` (`AIBlueprintHelperLibrary.GetAIController` self)) "Dead"))))

(event `/Game/AIContent/NPC/Guard/I_AIHelper.IsStateChanged`
  (params (State :type "/Game/AIContent/NPC/Guard/States Enum" :default "NewEnumerator0"))
  (message `/Game/AIContent/NPC/Guard/I_AIHelper.IsStateChanged` (`SkeletalMeshComponent.GetAnimInstance` (`self.Mesh`)) State))

(event `/Game/AIContent/NPC/Guard/I_AIHelper.SetAimState`
  (params (NewAimState :type Boolean))
  (message `/Game/AIContent/NPC/Guard/I_AIHelper.SetAimState` (`SkeletalMeshComponent.GetAnimInstance` (`self.Mesh`)) NewAimState))

(event `/Game/AIContent/NPC/Guard/I_AIHelper.SetWalkSpeed`
  (params (State :type "/Game/AIContent/NPC/Guard/States Enum" :default "NewEnumerator0"))
  (set `CharacterMovementComponent.MaxWalkSpeed` (select `/Game/AIContent/NPC/Guard/States` State :`NewEnumerator0` 150.0 :`NewEnumerator1` 200.0 :`NewEnumerator2` 400.0 :`NewEnumerator3` 600.0 :!type "Float (single-precision)") (`self.CharacterMovement`)))

(event `/Game/AIContent/NPC/Guard/I_AIHelper.TryShootEquipWeapon`
  (bind _weapon (`self.Weapon`)
    (:`then`
      (`/Game/AIContent/NPC/Classes/BP_WeaponBase.FireReguest` _weapon))
    (:`else`)))

(fn `GetPatrolRoute`
  (returns (PatrolRoute :type "/Game/AIContent/NPC/Guard/PatrolRoute Object Reference"))
  (return (`self.CustomPatrolPath`)))

(fn `GetTeamId`
  (returns (IsPlayer :type Boolean))
  (return false))

(fn `GetWeapon`
  (returns (HasWeapon :type Boolean) (Weapon :type "/Game/AIContent/NPC/Classes/BP_WeaponBase Object Reference"))
  (bind _weapon (`self.Weapon`))
  (return (`KismetSystemLibrary.IsValid` _weapon) _weapon))

(fn `GetWeaponRange`
  (returns (Range :type "Float (double-precision)"))
  (return (`/Game/AIContent/NPC/Classes/BP_WeaponBase.WeaponRange` (`self.Weapon`))))

(fn `IsDead`
  (returns (GetIsDead :type Boolean))
  (return (`/Game/AIContent/NPC/Guard/HealthComponent.isDead` (`self.HealthComponent`))))

(fn `UserConstructionScript`)